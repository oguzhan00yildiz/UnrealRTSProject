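; BP_Shop is an actor that awards money when its Box component is overlapped and shows the total on screen.
; On BeginPlay it casts and stores a WB_UI reference, uses it to create the widget, and adds that to the viewport.
; Each Box overlap, unfiltered by actor, prints a debug message, adds a fixed amount to Money and passes the total to the widget's UpdateScoreText.
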(event OnComponentBeginOverlap(Box)
  (params (OverlappedComponent :type Primitive%20Component%20Object%20Reference) (OtherActor :type Actor%20Object%20Reference) (OtherComp :type Primitive%20Component%20Object%20Reference) (OtherBodyIndex :type Integer) (bFromSweep :type Boolean) (SweepResult :type Hit%20Result%20Structure%20%28by%20ref%29))
  (Development|PrintString "Triggered" true false)
  (bind _output_get (Variables|Default|SetMoney (+ (Variables|Default|GetMoney) 10)))
  (Default|UpdateScoreText (stale EventBeginPlay _returnvalue) _output_get))

(event EventBeginPlay
  ;[0.15 0.15 0.15 0.5] Creating UI
  (bind _aswb_ui (Utilities|Casting|CastToWB_UIClass "/Game/Custom/BluePrints/WB_UI.WB_UI_C"))
  (Variables|Default|SetUIReference _aswb_ui)
  (bind _returnvalue (UserInterface|CreateWidget (Variables|Default|GetUIReference)))
  (UserInterface|Viewport|AddtoViewport _returnvalue 0))

(event Collision|EventActorBeginOverlap
  (params (OtherActor :type Actor%20Object%20Reference)))

(event EventTick
  (params (DeltaSeconds :type Float%20%28single-precision%29)))

(fn ConstructionScript)