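; BP_Spawner is an actor that spawns BP_Zombie instances around its own location at a regular interval.
; A looping timer started on BeginPlay fires StartSpawning, which offsets X and Y by a random unit vector scaled by SpawnRadius and keeps the spawner's Z.
; Each zombie then receives its default controller, with no spawn limit in the graph.
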(event Custom|StartSpawning
  (bind _returnvalue (Math|Random|RandomUnitVector))
  (bind _returnvalue_2 (Transformation|GetActorLocation))
  (bind _spawnradius (Variables|Default|GetSpawnRadius))
  (bind _returnvalue_3 (* _returnvalue _spawnradius))
  (bind _returnvalue_4 (+ _returnvalue_3 _returnvalue_2))
  (bind (_x _y) (Math|Vector|BreakVector _returnvalue_4))
  (bind _returnvalue_5 (Game|SpawnActorfromClass "/Game/Custom/BluePrints/BP_Zombie.BP_Zombie_C" (Math|Transform|MakeTransform (Math|Vector|MakeVector _x _y (.Z (Math|Vector|BreakVector _returnvalue_2)))) "Undefined" "MultiplyWithRoot" 0 0))
  (Pawn|SpawnDefaultController _returnvalue_5))

(event EventBeginPlay
  (Utilities|Time|SetTimerbyEvent (delegate Custom|StartSpawning) (Variables|Default|GetSpawnInterval) true))

(event Collision|EventActorBeginOverlap
  (params (OtherActor :type Actor%20Object%20Reference)))

(event EventTick
  (params (DeltaSeconds :type Float%20%28single-precision%29)))

(fn ConstructionScript)