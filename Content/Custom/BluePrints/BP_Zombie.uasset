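; BP_Zombie is an enemy zombie that pursues the player and dies after taking enough hits.
; Every tick it issues a simple move-to-actor order toward the first player character through its controller.
; Any actor overlap, with no type filter, flashes the mesh red briefly via a timer.
; When the timer fires, it restores the material, subtracts fixed damage, prints Health and destroys the actor at zero or below.
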(event Custom|FlashMaterial
  ;[0.15 0.15 0.15 0.5] GettingDamaged
  (Rendering|Material|SetMaterial (Variables|Character|GetMesh) 0 "/Game/Custom/Models/Zombie/parasitezombie_Material.parasitezombie_Material")
  (bind _output_get (Variables|Default|SetHealth (- (Variables|Default|GetHealth) 25)))
  (Development|PrintText (Utilities|Text|ToText(Integer) (Variables|Default|GetHealth)))
  (if (<= _output_get 0)
    (Actor|DestroyActor)))

(event EventBeginPlay)

(event Collision|EventActorBeginOverlap
  (params (OtherActor :type Actor%20Object%20Reference))
  ;[0.15 0.15 0.15 0.5] GettingDamaged
  (Rendering|Material|SetMaterial (Variables|Character|GetMesh) 0 "/Game/Custom/Materials/Red.Red")
  (Utilities|Time|SetTimerbyEvent (delegate Custom|FlashMaterial) 0.1))

(event EventTick
  (params (DeltaSeconds :type Float%20%28single-precision%29))
  ;[0.15 0.15 0.15 0.5] Movement
  (AI|Navigation|SimpleMovetoActor (Pawn|GetController) (Game|GetPlayerCharacter 0)))

(fn ConstructionScript)